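; Player character for a "carrinho de rolimã" downhill cart racer, with race start, braking, steering and a fail state that opens the test map.
; A velocity timeline drives MaxWalkSpeed and forward input, reversing while braking.
; Left/right timelines open Tick gates that add sideways input; E yaws the mesh.
; A dynamic material instance takes a colour and an enum-selected wood mask, reapplied every Tick through the Material_Carrinho graph.
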(event Custom|Value_Set
  ;[1 0.8141 0.2292] Material (INST)
  (Rendering|Material|SetVectorParameterValue (stale EventBeginPlay _returnvalue) "Color_Mask" (Utilities|Struct|MakeLinearColor (Variables|Personalização|GetColor_R) (Variables|Personalização|GetColor_G) (Variables|Personalização|GetColor_B) 1.0) :!class /Script/Engine.MaterialInstanceDynamic))

(event Custom|Break_OFF
  ;[1 1 1] Break/Brake
  (if (Variables|Carrinho|GetRace_Start?)
    (Variables|Carrinho|SetBreak? false)
    (Utilities|FlowControl|Sequence
      (:then_0
        (bind _value_brake_up (Timeline|Brake_Update Stop)
          (:Update
            (Variables|Carrinho|SetBrake_Velocidade_Car (/ _value_brake_up 1e+02)))
          (:Finished
            (Variables|Carrinho|SetBrake_Acabou true)
            ;[1 1 1] Tick (Update)
            (bind _speed_car (Timeline|Update_Velocity Play)
              (:Update
                (bind _output_get (Variables|/Script/Engine.CharacterMovementComponent|SetMaxWalkSpeed (Variables|Character|GetCharacterMovement) _speed_car))
                (Development|PrintString (Utilities|String|ToString(Float) _output_get) true true "(R=1.000000,G=0.026704,B=0.000000,A=1.000000)")
                (Pawn|Input|AddMovementInput (Math|Vector|GetForwardVector (Class|KismetMathLibrary|MakeRot 0.0 (.Yaw (Class|KismetMathLibrary|BreakRot (Pawn|GetControlRotation :!class /Script/Engine.Pawn))) 0.0)) 1.0 false)
                (if (<= _output_get 0.0)
                  (CallFunction|CarVelocity0 self)))))))
      (:then_1
        (Timeline|Update_Velocity Play)))))

(event Custom|Break_ON
  ;[1 1 1] Break/Brake
  (if (Variables|Carrinho|GetRace_Start?)
    (Variables|Carrinho|SetBreak? true)
    (Utilities|FlowControl|Sequence
      (:then_0
        (bind _value_brake_up (Timeline|Brake_Update Play)
          (:Update
            (Variables|Carrinho|SetBrake_Velocidade_Car (/ _value_brake_up 1e+02)))
          (:Finished
            (Variables|Carrinho|SetBrake_Acabou true)
            ;[1 1 1] Tick (Update)
            (bind _speed_car (Timeline|Update_Velocity Play)
              (:Update
                (bind _output_get (Variables|/Script/Engine.CharacterMovementComponent|SetMaxWalkSpeed (Variables|Character|GetCharacterMovement) _speed_car))
                (Development|PrintString (Utilities|String|ToString(Float) _output_get) true true "(R=1.000000,G=0.026704,B=0.000000,A=1.000000)")
                (Pawn|Input|AddMovementInput (Math|Vector|GetForwardVector (Class|KismetMathLibrary|MakeRot 0.0 (.Yaw (Class|KismetMathLibrary|BreakRot (Pawn|GetControlRotation :!class /Script/Engine.Pawn))) 0.0)) 1.0 false)
                (if (<= _output_get 0.0)
                  (CallFunction|CarVelocity0 self)))))))
      (:then_1
        (Timeline|Update_Velocity Reverse)))))

(event Custom|Rotation_Left
  (Variables|Default|SetRotation_Camera (Class|KismetMathLibrary|MakeRot 0.0 (+ (Variables|Default|GetRotation_Camera_F) 5.0) 0.0))
  (Transformation|AddRelativeRotation (Variables|Default|GetSpringArm) (Variables|Default|GetRotation_Camera) false))

(event Custom|Rotation_Right
  (Variables|Default|SetRotation_Camera (Class|KismetMathLibrary|MakeRot 0.0 (- (Variables|Default|GetRotation_Camera_F) 5.0) 0.0))
  (Transformation|AddRelativeRotation (Variables|Default|GetSpringArm) (Variables|Default|GetRotation_Camera) false))

(event Custom|Direita_OFF
  ;[0.135 0.135 1] Rotation
  (bind _output_get (Variables|Car_Var|SetDireita_F false))
  (bind _value_lr (Timeline|Left_Right_01 Reverse)
    (:Update
      (Utilities|FlowControl|Gate true) ; enters at Open
    )))

(event Custom|Esquerda_OFF
  ;[0.135 0.135 1] Rotation
  (bind _output_get (Variables|Car_Var|SetEsquerda_F false))
  (bind _value_lr (Timeline|Timeline_0 Reverse)
    (:Update
      (Utilities|FlowControl|Gate true) ; enters at Open
    )))

(event Custom|Esquerda
  ;[0.135 0.135 1] Rotation
  (if (Variables|Carrinho|GetRace_Start?)
    (Variables|Car_Var|SetEsquerda_F true)
    (bind _value_lr (Timeline|Timeline_0 Play)
      (:Update
        (Utilities|FlowControl|Gate true) ; enters at Open
      ))))

(event Custom|Direita
  ;[0.135 0.135 1] Rotation
  (if (Variables|Carrinho|GetRace_Start?)
    (Variables|Car_Var|SetDireita_F true)
    (bind _value_lr (Timeline|Left_Right_01 Play)
      (:Update
        (Utilities|FlowControl|Gate true) ; enters at Open
      ))))

(event Custom|Start_Race
  ;[1 1 1] Tick (Update)
  ;;[1 0 0] Start "Event"
  (Variables|Carrinho|SetRace_Start? true)
  (bind _speed_car (Timeline|Update_Velocity Play)
    (:Update
      (bind _output_get (Variables|/Script/Engine.CharacterMovementComponent|SetMaxWalkSpeed (Variables|Character|GetCharacterMovement) _speed_car))
      (Development|PrintString (Utilities|String|ToString(Float) _output_get) true true "(R=1.000000,G=0.026704,B=0.000000,A=1.000000)")
      (Pawn|Input|AddMovementInput (Math|Vector|GetForwardVector (Class|KismetMathLibrary|MakeRot 0.0 (.Yaw (Class|KismetMathLibrary|BreakRot (Pawn|GetControlRotation :!class /Script/Engine.Pawn))) 0.0)) 1.0 false)
      (if (<= _output_get 0.0)
        (CallFunction|CarVelocity0 self)))))

(event Custom|Car_Velocity_0
  ;[1 1 1] Tick (Update)
  ;[1 1 1] Break/Brake
  (bind _value_brake_up (Timeline|Brake_Update Stop)
    (:Update
      (Variables|Carrinho|SetBrake_Velocidade_Car (/ _value_brake_up 1e+02)))
    (:Finished
      (Variables|Carrinho|SetBrake_Acabou true)
      (bind _speed_car (Timeline|Update_Velocity Play)
        (:Update
          (bind _output_get (Variables|/Script/Engine.CharacterMovementComponent|SetMaxWalkSpeed (Variables|Character|GetCharacterMovement) _speed_car))
          (Development|PrintString (Utilities|String|ToString(Float) _output_get) true true "(R=1.000000,G=0.026704,B=0.000000,A=1.000000)")
          (Pawn|Input|AddMovementInput (Math|Vector|GetForwardVector (Class|KismetMathLibrary|MakeRot 0.0 (.Yaw (Class|KismetMathLibrary|BreakRot (Pawn|GetControlRotation :!class /Script/Engine.Pawn))) 0.0)) 1.0 false)
          (if (<= _output_get 0.0)
            (CallFunction|CarVelocity0 self)))))))

(event Custom|Corrida_Fail
  ;[1 1 1] Morreu
  (Utilities|FlowControl|Delay 0.2)
  (Development|PrintString "Perdi Acorrida")
  (Utilities|FlowControl|Sequence
    (:then_0
      ;[1 1 1] Tick (Update)
      (bind _speed_car (Timeline|Update_Velocity Stop)
        (:Update
          (bind _output_get (Variables|/Script/Engine.CharacterMovementComponent|SetMaxWalkSpeed (Variables|Character|GetCharacterMovement) _speed_car))
          (Development|PrintString (Utilities|String|ToString(Float) _output_get) true true "(R=1.000000,G=0.026704,B=0.000000,A=1.000000)")
          (Pawn|Input|AddMovementInput (Math|Vector|GetForwardVector (Class|KismetMathLibrary|MakeRot 0.0 (.Yaw (Class|KismetMathLibrary|BreakRot (Pawn|GetControlRotation :!class /Script/Engine.Pawn))) 0.0)) 1.0 false)
          (if (<= _output_get 0.0)
            (CallFunction|CarVelocity0 self)))))
    (:then_1
      ;[1 1 1] Break/Brake
      (bind _value_brake_up (Timeline|Brake_Update Stop)
        (:Update
          (Variables|Carrinho|SetBrake_Velocidade_Car (/ _value_brake_up 1e+02)))
        (:Finished
          (Variables|Carrinho|SetBrake_Acabou true)
          (Timeline|Update_Velocity Play))))
    (:then_2
      (Utilities|FlowControl|Delay 0.2)
      (Game|OpenLevel(byName) "Mapa_teste_game"))))

(event EventTick
  (params (DeltaSeconds :type Float%20%28single-precision%29))
  (bind _returnvalue (Pawn|GetControlRotation :!class /Script/Engine.Pawn))
  (bind _float_value_carrinho_rot (Variables|Carrinho|GetFloat_Value_Carrinho_Rot))
  (bind _yaw (Class|KismetMathLibrary|BreakRot _returnvalue))
  (bind _returnvalue_2 (Class|KismetMathLibrary|MakeRot 0.0 _yaw 0.0))
  (bind _returnvalue_3 (Math|Vector|GetRightVector _returnvalue_2))
  ;[1 0 0] Tick
  (Utilities|FlowControl|Sequence
    (:then_0
      ;[1 1 1] Tick (Update)
      (if (not (Variables|Personalização|GetInPersonalização))
        (if (Variables|Carrinho|GetBreak?)
          _)))
    (:then_1
      ;[1 0.8141 0.2292] Material (INST)
      (Utilities|MaterialCarrinho (stale EventBeginPlay _returnvalue)) ; enters at Tick
    )
    (:then_3
      ;[0.135 0.135 1] Rotation
      (Utilities|FlowControl|Sequence
        (:then_0
          (Utilities|FlowControl|Gate true :!label _label
            (:Exit
              (Utilities|FlowControl|Sequence
                (:then_0
                  (Variables|Carrinho|Setleft_Right (stale Custom|Direita_OFF _value_lr))
                  (Utilities|FlowControl|Delay 0.3))
                (:then_1
                  (if (stale Custom|Direita_OFF _output_get)
                    (Utilities|FlowControl|Delay 0.09)
                    (Pawn|Input|AddMovementInput _returnvalue_3 (* -2.0 _float_value_carrinho_rot) false)
                    (else
                      (goto _label Close))))))))
        (:then_1
          (Utilities|FlowControl|Gate true :!label _label_2
            (:Exit
              (Utilities|FlowControl|Sequence
                (:then_0
                  (Variables|Carrinho|Setleft_Right (stale Custom|Esquerda_OFF _value_lr))
                  (Utilities|FlowControl|Delay 0.3))
                (:then_1
                  (if (stale Custom|Esquerda_OFF _output_get)
                    (Utilities|FlowControl|Delay 0.09)
                    (Pawn|Input|AddMovementInput _returnvalue_3 (* 2.0 _float_value_carrinho_rot) false)
                    (else
                      (goto _label_2 Close))))))))))))

(event EventBeginPlay
  ;[1 0 0] Begin Play
  (Utilities|FlowControl|Sequence
    (:then_0
      ;[1 0.8141 0.2292] Material (INST)
      (bind _returnvalue (Rendering|Material|CreateDynamicMaterialInstance (Variables|Character|GetMesh) 0 0 :!class /Script/Engine.PrimitiveComponent))
      (Variables|Personalização|SetMaterial_Instance_Car _returnvalue)
      (Utilities|MaterialCarrinho _returnvalue))
    (:then_3
      ;[1 1 1] Tick (Update)
      (if (Variables|Personalização|GetInPersonalização)
        _))))

(event Input|AxisEvents|InputAxisMoveRight
  (params (AxisValue :type Float%20%28single-precision%29))
  ;[0.135 0.135 1] Rotation
)

(event Input|KeyboardEvents|E
  ;[0.135 0.135 1] Rotation
  (:Pressed
    (bind _yaw_value (Timeline|Giro Play)
      (:Update
        (Transformation|SetRelativeRotation (Variables|Character|GetMesh) (Class|KismetMathLibrary|MakeRot 0.0 _yaw_value 0.0) true))))
  (:Released
    (Timeline|Giro Reverse)))

(fn ConstructionScript)