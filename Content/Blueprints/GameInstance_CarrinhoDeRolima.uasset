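; Game instance for a soapbox-cart (carrinho de rolimã) game that holds and persists player progress: money, name, experience, rank, material choice and an account flag.
; Save, Load and Reset events call functions that copy these values to or from a Save_Game object in a single fixed slot.
; Reset loads the current save into the instance, writes a blank save over it, then quits the game.
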(event Custom|Reset_Game
  (CallFunction|ResetGameR))

(event Custom|Save_Game
  (Utilities|SaveGameS))

(event Custom|Load_Game
  (Utilities|LoadGameL))

(fn ResetGameR
  (bind _returnvalue (SaveGame|LoadGamefromSlot "1"))
  (bind _assave_game (Utilities|Casting|CastToSave_Game _returnvalue)
    (:then
      (Variables|Default|SetMoney (Variables|/Game/SaveGame/Save_Game.Save_Game_C|GetMoney _assave_game))
      (Variables|Default|SetPlayer_Name (Variables|/Game/SaveGame/Save_Game.Save_Game_C|GetPlayer_Name _assave_game))
      (Variables|Default|SetEXP (Variables|/Game/SaveGame/Save_Game.Save_Game_C|GetEXP _assave_game))
      (Variables|Default|SetLevelRank (Variables|/Game/SaveGame/Save_Game.Save_Game_C|GetLevelRank _assave_game))
      (Variables|Default|SetNumero_do_Material (Variables|/Game/SaveGame/Save_Game.Save_Game_C|GetNumero_do_Material _assave_game))
      (Variables|Default|SetConta? (Variables|/Game/SaveGame/Save_Game.Save_Game_C|GetConta? _assave_game))
      (bind _returnvalue_2 (SaveGame|CreateSaveGameObject "/Game/SaveGame/Save_Game.Save_Game_C"))
      (bind _assave_game_2 (Utilities|Casting|CastToSave_Game _returnvalue_2)
        (:then
          (Variables|/Game/SaveGame/Save_Game.Save_Game_C|SetMoney _assave_game_2 0.0)
          (Variables|/Game/SaveGame/Save_Game.Save_Game_C|SetPlayer_Name _assave_game_2 "")
          (Variables|/Game/SaveGame/Save_Game.Save_Game_C|SetEXP _assave_game_2 0.0)
          (Variables|/Game/SaveGame/Save_Game.Save_Game_C|SetLevelRank _assave_game_2 0)
          (Variables|/Game/SaveGame/Save_Game.Save_Game_C|SetNumero_do_Material _assave_game_2 "NewEnumerator0")
          (Variables|/Game/SaveGame/Save_Game.Save_Game_C|SetConta? _assave_game_2 false)
          (SaveGame|SaveGametoSlot _assave_game_2 "1")
          (Game|QuitGame (Game|GetPlayerController 0) "Quit"))
        (:CastFailed
          _)))
    (:CastFailed
      _))
  (return))