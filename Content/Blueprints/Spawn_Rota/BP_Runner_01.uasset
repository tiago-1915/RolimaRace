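; BP_Runner_01 is a floor tile for an endless runner starring the CarrinhoDeRolima player.
; Its construction script scatters ten child actors inside the CoinArea box as coins and places one car at a random choice of four spawn points.
; When the player overlaps EndTrigger, the tile asks the game mode to add another tile, then destroys itself after a short delay.
; GetAttachTransform exposes the AttachPoint transform; a failed self-spawning attempt remains disconnected.
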(event OnComponentBeginOverlap(EndTrigger)
  (params (OtherActor :type Actor%20Object%20Reference) (OtherComp :type Primitive%20Component%20Object%20Reference) (OtherBodyIndex :type Integer) (bFromSweep :type Boolean) (SweepResult :type Hit%20Result%20Structure%20%28by%20ref%29))
  (Utilities|Casting|CastToCarrinhoDeRolima_01_Player OtherActor)
  (bind _asgame_mode_carrinho_de_rolima (Utilities|Casting|CastToGameMode_CarrinhoDeRolima (Game|GetGameMode)))
  (Default|AddFloorTile _asgame_mode_carrinho_de_rolima)
  (Utilities|FlowControl|Delay 0.2)
  (Actor|DestroyActor self))

(event EventBeginPlay)

(event Collision|EventActorBeginOverlap
  (params (OtherActor :type Actor%20Object%20Reference)))

(event EventTick
  (params (DeltaSeconds :type Float%20%28single-precision%29)))

(fn ConstructionScript
  (CallFunction|SetSpawnPoints)
  (CallFunction|SpawnCoins)
  (CallFunction|SpawnCar))

(fn GetAttachTransform
  (return (Transformation|GetWorldTransform (Variables|Default|GetAttachPoint))))

(fn SetSpawnPoints
  (Variables|Default|SetSpawnPoints (Utilities|Array|MakeArray (Transformation|GetRelativeTransform (Variables|Default|GetCarSpawnPointL)) (Transformation|GetRelativeTransform (Variables|Default|GetCarSpawnPointR)) (Transformation|GetRelativeTransform (Variables|Default|GetCarSpawnPointL2)) (Transformation|GetRelativeTransform (Variables|Default|GetCarSpawnPointR2)))))

(fn SpawnCar
  (bind _spawnpoints (Variables|Default|GetSpawnPoints))
  (AddComponent|AddChildActorComponent false (Utilities|Array|Get(acopy) _spawnpoints (Math|Random|RandomIntegerinRange 0 (Utilities|Array|LastIndex _spawnpoints)))))

(fn SpawnCoins
  (bind _coinarea (Variables|Default|GetCoinArea))
  (for _index (range 0 9)
    (AddComponent|AddChildActorComponent false (Math|Conversions|ToTransform(Vector) (Math|Random|RandomPointinBoundingBox (Variables|/Script/Engine.SceneComponent|GetRelativeLocation _coinarea) (Variables|/Script/Engine.BoxComponent|GetBoxExtent _coinarea))))))